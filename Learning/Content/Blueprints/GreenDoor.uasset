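; GreenDoor is an interactive painted wooden door that swings open or shut when E is pressed nearby.
; Overlap begin and end enable and disable input from player controller 0, without checking which actor overlaps.
; The E key plays or reverses the Opendoor timeline, which drives the mesh's relative yaw.
; Tick derives IsClosed from the timeline value to choose the direction.
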(event EventBeginPlay)

(event EventTick
  (params (DeltaSeconds :type Float%20%28single-precision%29))
  (Variables|Default|SetIs%20closed (< (stale Input|KeyboardEvents|E _newtrack_0) 1.0)))

(event Collision|EventActorBeginOverlap
  (params (OtherActor :type Actor%20Object%20Reference))
  (Input|EnableInput (Game|GetPlayerController 0)))

(event Collision|EventActorEndOverlap
  (params (OtherActor :type Actor%20Object%20Reference))
  (Input|DisableInput (Game|GetPlayerController 0)))

(event Input|KeyboardEvents|E
  (params (Key :type Key%20Structure :default "None"))
  (:Pressed
    (if (Variables|Default|GetIs%20closed)
      (bind _newtrack_0 (Timeline|opendoor Play)
        (:Update
          (Transformation|SetRelativeRotation (Variables|Default|GetS_Painted_Wooden_Door_vmqifgedw_lod3_Var3) (Math|Rotator|MakeRotator 0.0 0.0 _newtrack_0) false false)))
      (else
        (Timeline|opendoor Reverse)))))

(fn ConstructionScript)